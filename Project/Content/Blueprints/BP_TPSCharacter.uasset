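; BP_TPSCharacter is the player character Blueprint for a third-person shooter, linking the character to its UI.
; On BeginPlay it creates the HUD widget, then after a short delay fills in health and sets the default weapon display.
; UIshowHP writes the health ratio and text to the HUD, and OnUsingGrenade swaps its weapon indicator.
; OnGameOver calls the parent, shows the mouse cursor and opens the game-over screen.
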(event `self.OnGameOver`
  (`parent.OnGameOver`)
  (set `PlayerController.bShowMouseCursor` true (`GameplayStatics.GetPlayerController` 0))
  (bind _returnvalue (`|CreateWidget` "/Game/Blueprints/UI_GameOver.UI_GameOver_C"))
  (`UserWidget.AddToViewport` _returnvalue 0))

(event `self.OnUsingGrenade`
  (params (isGrenade :type Boolean))
  (bind _uiscreen (`self.UIScreen`))
  (`/Engine/EditorBlueprintResources/StandardMacros.IsValid` _uiscreen
    (:`Is Valid`
      (set `/Game/Blueprints/UI_Screen.isGrenaded` isGrenade _uiscreen)
      (`/Game/Blueprints/UI_Screen.SwapWeapon` _uiscreen))))

(event `self.ReceiveBeginPlay`
  (bind _returnvalue (`|CreateWidget` "/Game/Blueprints/UI_Screen.UI_Screen_C" (`GameplayStatics.GetPlayerController` 0)))
  (bind _output_get (set `self.UIScreen` _returnvalue))
  (`UserWidget.AddToViewport` _output_get 0)
  (`KismetSystemLibrary.Delay` 0.05)
  (`self.UIshowHP`)
  (`self.OnUsingGrenade` false))

(fn `UIshowHP`
  (bind _hp (`self.hp`))
  (bind _initialhp (`self.initialHP`))
  (bind _uiscreen (`self.UIScreen`))
  (set `/Game/Blueprints/UI_Screen.hpRatio` (/ (`KismetMathLibrary.Conv_IntToDouble` _hp) (`KismetMathLibrary.Conv_IntToDouble` _initialhp)) _uiscreen)
  (set `/Game/Blueprints/UI_Screen.hpString` (`KismetStringLibrary.Concat_StrStr` (`KismetStringLibrary.Conv_IntToString` _hp) "/" (`KismetStringLibrary.Conv_IntToString` _initialhp)) _uiscreen))

(fn `UserConstructionScript`)